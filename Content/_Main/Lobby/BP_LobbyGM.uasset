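; Lobby game mode that registers joining players and initialises their lobby menu.
; On PostLogin it tracks the player, caches PlayerStart actors, and pulls server name and max players from the game instance.
; It then messages the lobby player controller to run initial setup and show the server name and default map settings.
; RespawnPlayer is called last but has no implementation yet.
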(event `self.K2_PostLogin`
  (params (NewPlayer :type "PlayerController Object Reference"))
  (bind _output_get (set `self.ConnectedPlayer` NewPlayer))
  (`KismetArrayLibrary.Array_AddUnique` (`self.Players`) _output_get)
  (bind _outactors (`GameplayStatics.GetAllActorsOfClass` "/Script/Engine.PlayerStart"))
  (set `self.SpawnPoints` _outactors)
  (bind _gameinstance (message `/Game/GameInstances/BPI_GameInstance.GameInstanceRef` (`GameplayStatics.GetGameInstance`)))
  (set `self.Server Name` (`/Game/GameInstances/MainMenuGameInstance.ServerName` _gameinstance))
  (set `self.Max Players` (`/Game/GameInstances/MainMenuGameInstance.MaxPlayers` _gameinstance))
  (bind _lobbypc (message `/Game/_Main/Lobby/BPI_LobbyPC.LobbyPCRef` (`self.ConnectedPlayer`)))
  (`/Game/_Main/Lobby/BP_LobbyPC.InitialSetup` _lobbypc)
  (`/Game/_Main/Lobby/BP_LobbyPC.SetupLobbyMenu` _lobbypc (`self.Server Name`))
  (`/Game/_Main/Lobby/BP_LobbyPC.UpdateLobbySettings` _lobbypc (`self.DefaultMapImage`) (`self.DefaultMapName`) (`self.DefaultMapTime`))
  (`self.RespawnPlayer` (`self.ConnectedPlayer`)))

(event `RespawnPlayer`
  (params (Player :type "PlayerController Object Reference")))

(fn `UserConstructionScript`)